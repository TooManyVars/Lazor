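; An actor that turns a chosen static mesh into a sliceable procedural mesh and cuts it in half on Breakmesh.
; The construction script copies MeshToCopy into the procedural mesh with collision, then destroys the static mesh component to avoid a duplicate.
; Breakmesh slices at the actor's location along a fixed Y-normal plane with a metal cap, enables physics on the new half, then destroys that half after a brief delay.
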(event `Break mesh`
  ;[1 1 1] Slice the procedural mesh in half and create a second procedural mesh.
  (bind _outotherhalfprocmesh (`KismetProceduralMeshLibrary.SliceProceduralMesh` (`self.ProceduralMesh`) (`self.K2_GetActorLocation`) (0.0 1.0 0.0) true "CreateNewSectionForCap" "/Game/StarterContent/Materials/M_Metal_Brushed_Nickel.M_Metal_Brushed_Nickel"))
  ;[1 1 1] The second procedural mesh created does not simulate physics as this must be set manually.
  (`PrimitiveComponent.SetSimulatePhysics` _outotherhalfprocmesh true)
  (`KismetSystemLibrary.Delay` 0.02)
  (`ActorComponent.K2_DestroyComponent` _outotherhalfprocmesh))

(event `self.ReceiveBeginPlay`)

(fn `UserConstructionScript`
  ;[1 1 1] Initilize and copy the static mesh to the procedural mesh. destroy the static mesh after to prevent having two meshes.
  (`StaticMeshComponent.SetStaticMesh` (`self.StaticMesh`) (`self.MeshToCopy`))
  (`KismetProceduralMeshLibrary.CopyProceduralMeshFromStaticMeshComponent` (`self.StaticMesh`) 0 (`self.ProceduralMesh`) true)
  (`ActorComponent.K2_DestroyComponent` (`self.StaticMesh`)))